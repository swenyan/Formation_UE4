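; RTS camera pawn that selects TpsCharacter_BP units and moves them in grid formations through RTS_AI_Controller.
; Clicking selects a unit (Shift adds, Q selects all) or sends the selection to the clicked point, while number keys change column count.
; Grid slots alternate either side of the anchor on both axes; a line-formation helper is unused.
; BeginPlay selects all units and endlessly cycles column counts and anchor shifts on timed delays.
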(event `self.ReceiveBeginPlay`
  (set `PlayerController.bShowMouseCursor` true (`GameplayStatics.GetPlayerController` 0))
  (set `self.ActorZeroLocation` (`self.K2_GetActorLocation`))
  (bind _outactors (`GameplayStatics.GetAllActorsOfClass` "/Game/TpsCharacter_BP.TpsCharacter_BP_C"))
  (set `self.SelectedActors` _outactors)
  (`KismetSystemLibrary.Delay` 4.0 :!label _label)
  (set `self.TotalCol` 3)
  (`self.Move In Formation`)
  (`KismetSystemLibrary.Delay` 4.0)
  (set `self.TotalCol` 5)
  (`self.Move In Formation`)
  (`KismetSystemLibrary.Delay` 4.0)
  (set `self.ActorZeroLocation` (+ (`self.ActorZeroLocation`) (0.0 1000.0 0.0)))
  (`self.Move In Formation`)
  (set `self.ActorZeroLocation` (`self.K2_GetActorLocation`))
  (`KismetSystemLibrary.Delay` 4.0)
  (set `self.TotalCol` 6)
  (`self.Move In Formation`)
  (`KismetSystemLibrary.Delay` 4.0)
  (set `self.ActorZeroLocation` (+ (`self.ActorZeroLocation`) (0.0 -1000.0 0.0)))
  (`self.Move In Formation`)
  (set `self.ActorZeroLocation` (`self.K2_GetActorLocation`))
  (`KismetSystemLibrary.Delay` 4.0)
  (set `self.TotalCol` 10)
  (`self.Move In Formation`)
  (`KismetSystemLibrary.Delay` 4.0)
  (set `self.TotalCol` 15)
  (`self.Move In Formation`)
  (goto _label))

(event `InputAxis|MoveForward`
  (params (AxisValue :type "Float (single-precision)"))
  (`PawnMovementComponent.AddInputVector` (`self.FloatingPawnMovement`) (* (`KismetMathLibrary.GetForwardVector` (`self.K2_GetActorRotation`)) AxisValue) false))

(event `InputAxis|MoveRight`
  (params (AxisValue :type "Float (single-precision)"))
  (`PawnMovementComponent.AddInputVector` (`self.FloatingPawnMovement`) (* (`KismetMathLibrary.GetRightVector` (`self.K2_GetActorRotation`)) AxisValue) false))

(event `Key|LeftMouseButton`
  (params (Key :type "Key Structure"))
  (bind _selectedactors (`self.SelectedActors`))
  (bind (_hitresult _returnvalue) (`PlayerController.GetHitResultUnderCursorByChannel` (`GameplayStatics.GetPlayerController` 0) "TraceTypeQuery1" true))
  (bind (_bblockinghit _binitialoverlap _time _distance _location _impactpoint _normal _impactnormal _physmat _hitactor) (`GameplayStatics.BreakHitResult` _hitresult))
  (:`Pressed`
    (if _returnvalue
      (set `self.ActorZeroLocation` _location)
      (bind _astps_character_bp (cast `/Game/TpsCharacter_BP` _hitactor)
        (:`then`
          (if (`self.IsMultiSelect`)
            (`KismetArrayLibrary.Array_AddUnique` _selectedactors _astps_character_bp)
            (else
              (`KismetArrayLibrary.Array_Clear` _selectedactors)
              (`KismetArrayLibrary.Array_Set` _selectedactors 0 _astps_character_bp true))))
        (:`CastFailed`
          (`self.Move In Formation`))))))

(event `Key|LeftShift`
  (params (Key :type "Key Structure"))
  ;[1 1 1] 按住左Shift选择多个单位
  (:`Pressed`
    (set `self.IsMultiSelect` true))
  (:`Released`
    (set `self.IsMultiSelect` false)))

(event `Move In Formation`
  (for (_array_element _array_index) (`self.SelectedActors`)
    (if (!= _array_element null)
      (bind _asrts_ai_controller (cast `/Game/RTS_AI_Controller` (`AIBlueprintHelperLibrary.GetAIController` _array_element)))
      (`AIController.MoveToLocation` _asrts_ai_controller (`self.GetQuadFormationPosition` (`self.ActorZeroLocation`) _array_index (`self.TotalCol`) 200.0 200.0) 0.0 false true true true null true))))

(event `Key|Q`
  (params (Key :type "Key Structure"))
  (:`Pressed`
    (bind _outactors (`GameplayStatics.GetAllActorsOfClass` "/Game/TpsCharacter_BP.TpsCharacter_BP_C"))
    (set `self.SelectedActors` _outactors)))

(event `Key|One`
  (params (Key :type "Key Structure"))
  (:`Pressed`
    (set `self.TotalCol` 2)
    (`self.Move In Formation`)))

(event `Key|Two`
  (params (Key :type "Key Structure"))
  (:`Pressed`
    (set `self.TotalCol` 3)
    (`self.Move In Formation`)))

(event `Key|Three`
  (params (Key :type "Key Structure"))
  (:`Pressed`
    (set `self.TotalCol` 5)
    (`self.Move In Formation`)))

(event `Key|Four`
  (params (Key :type "Key Structure"))
  (:`Pressed`
    (set `self.TotalCol` 6)
    (`self.Move In Formation`)))

(event `Key|Five`
  (params (Key :type "Key Structure"))
  (:`Pressed`
    (set `self.TotalCol` 10)
    (`self.Move In Formation`)))

(event `Key|Six`
  (params (Key :type "Key Structure"))
  (:`Pressed`
    (set `self.TotalCol` 15)
    (`self.Move In Formation`)))

(fn `GetFormationOffsetByIndex`
  (params (OffsetStep :type "Float (double-precision)") (Index :type Integer))
  (returns (Result :type "Float (double-precision)"))
  (locals (var_index :type Integer) (var_offset :type "Float (double-precision)"))
  (set `local.var_index` Index)
  (set `local.var_offset` OffsetStep)
  (if (== (mod Index 2) 0)
    (return (* (/ (`local.var_index`) 2) (`local.var_offset`)))
    (else
      (return (* (/ (+ (`local.var_index`) 1) 2) (* (`local.var_offset`) -1.0))))))

(fn `GetLineFormationPosition`
  (params (ActorZeroLocation :type "Vector Structure") (OffsetBetweenActors :type "Float (double-precision)") (ActorIndex :type Integer))
  (returns (Position :type "Vector Structure"))
  (locals (FormationPosition :type "Vector Structure") (ZeroLocation :type "Vector Structure") (Offset :type "Float (double-precision)") (Index :type Integer))
  (set `local.ZeroLocation` ActorZeroLocation)
  (set `local.Offset` OffsetBetweenActors)
  (set `local.Index` ActorIndex)
  (`|ExecutionSequence`
    (:`then_0`
      (if (== (`local.Index`) 0)
        (set `local.FormationPosition` (`local.ZeroLocation`))
        (else
          (set `local.FormationPosition` (`KismetMathLibrary.MakeVector` (.x (`local.ZeroLocation`)) (+ (`self.GetFormationOffsetByIndex` (`local.Offset`) (`local.Index`)) (.y (`local.ZeroLocation`))) (.z (`local.ZeroLocation`)))))))
    (:`then_1`
      (return (`local.FormationPosition`)))))

(fn `GetQuadFormationPosition`
  (params (`Actor Zero Location` :type "Vector Structure") (Index :type Integer) (TotalCol :type Integer) (RowOffsetFactor :type "Float (double-precision)") (ColOffsetFactor :type "Float (double-precision)"))
  (returns (Location :type "Vector Structure"))
  (locals (Var_Row :type Integer) (Var_Col :type Integer) (Var_Index :type Integer) (Var_ZeroLocation :type "Vector Structure") (Var_RowOffsetFactor :type "Float (double-precision)") (Var_ColOffsetFactor :type "Float (double-precision)"))
  (if (== Index 0)
    (return `Actor Zero Location`)
    (else
      (`|ExecutionSequence`
        (:`then_0`
          (set `local.Var_ZeroLocation` `Actor Zero Location`))
        (:`then_1`
          (bind _output_get (set `local.Var_Index` Index))
          (set `local.Var_Col` (mod _output_get TotalCol)))
        (:`then_2`
          (set `local.Var_Row` (/ (`local.Var_Index`) TotalCol)))
        (:`then_3`
          (set `local.Var_RowOffsetFactor` RowOffsetFactor))
        (:`then_4`
          (set `local.Var_ColOffsetFactor` ColOffsetFactor))
        (:`then_5`
          (return (+ (`KismetMathLibrary.MakeVector` (`self.GetFormationOffsetByIndex` (`local.Var_RowOffsetFactor`) (`local.Var_Row`)) (`self.GetFormationOffsetByIndex` (`local.Var_ColOffsetFactor`) (`local.Var_Col`))) (`local.Var_ZeroLocation`))))))))

(fn `UserConstructionScript`)